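; BP_LevelSave is a save-game Blueprint that holds the level list with per-level solve state, plus the last level.
; GetLevel and GetSolveState turn a one-based level number into a clamped Levels index, though GetSolveState's upper clamp allows one past the final index.
; GetLevel also prints the level number.
; LastLevel and Levels have simple accessors, while SetSolveState is an empty stub.
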(fn `GetLastLevel`
  (returns (LastLevel :type Integer))
  (return (`self.LastLevel`)))

(fn `GetLevel`
  (params (LevelNumber :type Integer))
  (returns (Level :type "ChineseRoomLevel Class Reference"))
  (bind (_level _state _levelnumber) (break `LevelSave` (`|GetArrayItem` (`self.Levels`) (`KismetMathLibrary.Clamp` (- LevelNumber 1) 0 (- (`KismetArrayLibrary.Array_Length` (`self.Levels`)) 1)))))
  (`KismetSystemLibrary.PrintString` null (`KismetStringLibrary.Conv_IntToString` _levelnumber))
  (return _level))

(fn `GetLevels`
  (returns (Levels :type "Array of LevelSave Structure"))
  (return (`self.Levels`)))

(fn `GetSolveState`
  (params (LevelNumber :type Integer))
  (returns (State :type "ESolveState Enum"))
  (return (`.State` (break `LevelSave` (`|GetArrayItem` (`self.Levels`) (`KismetMathLibrary.Clamp` (- LevelNumber 1) 0 (- (`KismetArrayLibrary.Array_Length` (`self.Levels`)) 0)))))))

(fn `SetLastLevel`
  (params (LastLevel :type Integer))
  (set `self.LastLevel` LastLevel)
  (return))

(fn `SetSolveState`)